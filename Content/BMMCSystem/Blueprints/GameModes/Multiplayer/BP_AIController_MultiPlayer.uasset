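; Multiplayer AI controller that handles activation, death reporting and respawn for bot-controlled pawns.
; On possess it activates the pawn's components and sends it an AI begin-play message if the game state shows a match in progress.
; Death and respawn interface events, gated on local controller, pass to server-named events that report to the game state and request respawn from the game mode.
; Delay and team-variable getters return placeholder values.
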(event Custom|PlayerDeathSERVER
  ;[1 1 1 0.1] AI Death
  (bind _asbp_gs_multi_player (Utilities|Casting|CastToBP_GS_MultiPlayer (Game|GetGameState)))
  (Default|ReportDeath _asbp_gs_multi_player (Pawn|GetControlledPawn)))

(event Custom|RespawnPlayerSERVER
  ;[1 1 1 0.1] AI Respawn
  (bind _asbp_gm_multiplayer (Utilities|Casting|CastToBP_GM_Multiplayer (Game|GetGameMode)))
  (Default|RespawnAIEvent _asbp_gm_multiplayer self))

(event Custom|ActivatePlayerSERVER
  ;[1 1 1 0.1] Activate AI
  (CallFunction|ActivateComponents (Pawn|GetControlledPawn))
  (bind _asbp_gs_multi_player (Utilities|Casting|CastToBP_GS_MultiPlayer (Game|GetGameState)))
  (if (and (Variables|/Game/BMMCSystem/Blueprints/GameModes/Multiplayer/BP_GS_MultiPlayer.BP_GS_MultiPlayer_C|GetMatchStarted _asbp_gs_multi_player) (not (Variables|/Game/BMMCSystem/Blueprints/GameModes/Multiplayer/BP_GS_MultiPlayer.BP_GS_MultiPlayer_C|GetMatchEnded _asbp_gs_multi_player)))
    (Class|BPICharacters|IAIBeginPlay(Message) (Pawn|GetControlledPawn))))

(event Custom|ActivatePlayerCLIENT
  ;[1 1 1 0.1] Activate AI
  (CallFunction|ActivatePlayerSERVER))

(event EventPossess
  (params (PossessedPawn :type Pawn%20Object%20Reference))
  ;[1 1 1 0.1] Activate AI
  (CallFunction|ACtivatePlayerCLIENT))

(event EventIControllerDeathReport
  ;[1 1 1 0.1] AI Death
  (if (Pawn|IsLocalController)
    (CallFunction|PlayerDeathSERVER)))

(event EventIRespawn
  ;[1 1 1 0.1] AI Respawn
  (if (Pawn|IsLocalController)
    (CallFunction|RespawnPlayerSERVER)))

(fn ConstructionScript)

(fn IGetGameModeStartDelay
  (return 0.0))

(fn IGetTeamVariables
  (return "" "" 0))