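; BP_WeaponSpawner is a debug actor that spawns a pickable weapon at a random point inside a box when the multiplayer countdown starts.
; On the server, BeginPlay binds StartEvent to the BP_GM_Multiplayer countdown event, using a direct cast to avoid a delay.
; StartEvent spawns a BP_WeaponsBase with the configured WeaponName and initializes its weapon component through interfaces.
; The construction script sizes the spawn box from BoxSize.
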(event Custom|StartEvent
  (bind _spawnbox (Variables|Default|GetSpawnBox))
  (bind _returnvalue (Game|SpawnActorfromClass "/Game/BMMCSystem/Blueprints/Weapons/BP_WeaponsBase.BP_WeaponsBase_C" (Math|Transform|MakeTransform (Math|Random|RandomPointinBoundingBox (Transformation|GetWorldLocation _spawnbox) (Variables|/Script/Engine.BoxComponent|GetBoxExtent _spawnbox))) "AdjustIfPossibleButAlwaysSpawn" self (Variables|Default|GetWeaponName) 0))
  (if (Utilities|DoesObjectImplementInterface _returnvalue "/Game/BMMCSystem/Blueprints/Interfaces/BPI_Weapons.BPI_Weapons_C")
    (Class|BPIComponentsWeapons|IInitPickableWeapon(Message) (.Component (CallFunction|FGetWeaponComponent _returnvalue)) (Variables|Default|GetWeaponName))))

(event EventBeginPlay
  (if (Ability|HasAuthority)
    (bind _asbp_gm_multiplayer (Utilities|Casting|CastToBP_GM_Multiplayer (Game|GetGameMode))) ; Had to use cast here, to avoid a random delay
    (EventDispatchers|BindEventtoEDCountdownStarted _asbp_gm_multiplayer (delegate Custom|StartEvent))))

(fn ConstructionScript
  (Components|Box|SetBoxExtent (Variables|Default|GetSpawnBox) (Variables|Default|GetBoxSize) true))