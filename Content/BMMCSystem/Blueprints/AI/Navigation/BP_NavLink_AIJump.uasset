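; BP_NavLink_AIJump is a smart nav link that makes AI characters jump to the link's destination.
; When an agent reaches it, the link stops that character's AI movement and computes an arced launch velocity with SuggestProjectileVelocityCustomArc.
; It launches the character with that velocity, overriding current velocity, and turns it to face the horizontal direction of the jump.
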(event EventSmartLinkReached
  (params (Agent :type Actor%20Object%20Reference) (Destination :type Vector%20%28by%20ref%29 :default "0, 0, 0"))
  (Utilities|IsValid Agent
    (:Is%20Valid
      (bind _as캐릭터 (Utilities|Casting|CastToCharacter Agent))
      (AI|Navigation|StopMovement (AI|GetAIController _as캐릭터))
      (bind _outlaunchvelocity (Game|SuggestProjectileVelocityCustomArc (Transformation|GetActorLocation _as캐릭터) Destination 0.0 0.35))
      (Character|LaunchCharacter _as캐릭터 _outlaunchvelocity true true)
      (Transformation|SetActorRotation _as캐릭터 (Math|Conversions|RotationFromXVector (Math|Vector|MakeVector (.X (Math|Vector|BreakVector _outlaunchvelocity)) (.Y (Math|Vector|BreakVector _outlaunchvelocity)) 0.0))))))

(fn ConstructionScript)